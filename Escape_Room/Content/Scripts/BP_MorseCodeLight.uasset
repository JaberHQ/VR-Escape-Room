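; BP_MorseCodeLight blinks a point light in a repeating Morse-code-style pattern.
; From BeginPlay, a hardcoded chain of ToggleVisibility calls and Delays produces short and long intervals in three numbered groups separated by longer pauses.
; The chain loops back to its start indefinitely, with Retriggerable Delays at both ends and no variables or data driving the sequence.
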(event EventBeginPlay
  ;[0.15 0.15 0.15 0.5] 1
  (Utilities|FlowControl|RetriggerableDelay 1.0 :!label _label)
  (Rendering|ToggleVisibility (Variables|Default|GetPointLight) false)
  (Utilities|FlowControl|Delay 0.5)
  (Rendering|ToggleVisibility (Variables|Default|GetPointLight) false)
  (Utilities|FlowControl|Delay 1.0)
  (Rendering|ToggleVisibility (Variables|Default|GetPointLight) false)
  (Utilities|FlowControl|Delay 0.5)
  (Rendering|ToggleVisibility (Variables|Default|GetPointLight) false)
  (Utilities|FlowControl|Delay 0.5)
  (Rendering|ToggleVisibility (Variables|Default|GetPointLight) false)
  (Utilities|FlowControl|Delay 1.0)
  (Rendering|ToggleVisibility (Variables|Default|GetPointLight) false)
  (Utilities|FlowControl|Delay 0.5)
  (Rendering|ToggleVisibility (Variables|Default|GetPointLight) false)
  (Utilities|FlowControl|Delay 0.5)
  (Rendering|ToggleVisibility (Variables|Default|GetPointLight) false)
  (Utilities|FlowControl|Delay 0.2)
  (Rendering|ToggleVisibility (Variables|Default|GetPointLight) false)
  (Utilities|FlowControl|Delay 2.0)
  ;[0.15 0.15 0.15 0.5] 2
  (Rendering|ToggleVisibility (Variables|Default|GetPointLight) false)
  (Utilities|FlowControl|Delay 1.0)
  (Rendering|ToggleVisibility (Variables|Default|GetPointLight) false)
  (Utilities|FlowControl|Delay 0.5)
  (Rendering|ToggleVisibility (Variables|Default|GetPointLight) false)
  (Utilities|FlowControl|Delay 1.0)
  (Rendering|ToggleVisibility (Variables|Default|GetPointLight) false)
  (Utilities|FlowControl|Delay 0.5)
  (Rendering|ToggleVisibility (Variables|Default|GetPointLight) false)
  (Utilities|FlowControl|Delay 1.0)
  (Rendering|ToggleVisibility (Variables|Default|GetPointLight) false)
  (Utilities|FlowControl|Delay 0.5)
  (Rendering|ToggleVisibility (Variables|Default|GetPointLight) false)
  (Utilities|FlowControl|Delay 0.2)
  (Rendering|ToggleVisibility (Variables|Default|GetPointLight) false)
  (Utilities|FlowControl|Delay 0.5)
  (Rendering|ToggleVisibility (Variables|Default|GetPointLight) false)
  (Utilities|FlowControl|Delay 0.2)
  (Rendering|ToggleVisibility (Variables|Default|GetPointLight) false)
  (Utilities|FlowControl|Delay 2.0)
  ;[0.15 0.15 0.15 0.5] 3
  (Rendering|ToggleVisibility (Variables|Default|GetPointLight) false)
  (Utilities|FlowControl|Delay 1.0)
  (Rendering|ToggleVisibility (Variables|Default|GetPointLight) false)
  (Utilities|FlowControl|Delay 0.5)
  (Rendering|ToggleVisibility (Variables|Default|GetPointLight) false)
  (Utilities|FlowControl|Delay 0.2)
  (Rendering|ToggleVisibility (Variables|Default|GetPointLight) false)
  (Utilities|FlowControl|Delay 0.5)
  (Rendering|ToggleVisibility (Variables|Default|GetPointLight) false)
  (Utilities|FlowControl|Delay 1.0)
  (Rendering|ToggleVisibility (Variables|Default|GetPointLight) false)
  (Utilities|FlowControl|Delay 0.5)
  (Rendering|ToggleVisibility (Variables|Default|GetPointLight) false)
  (Utilities|FlowControl|Delay 0.2)
  (Rendering|ToggleVisibility (Variables|Default|GetPointLight) false)
  (Utilities|FlowControl|Delay 0.5)
  (Rendering|ToggleVisibility (Variables|Default|GetPointLight) false)
  (Utilities|FlowControl|Delay 0.2)
  (Rendering|ToggleVisibility (Variables|Default|GetPointLight) false)
  (Utilities|FlowControl|RetriggerableDelay 3.0)
  (Rendering|ToggleVisibility (Variables|Default|GetPointLight) false)
  (goto _label))

(fn ConstructionScript)